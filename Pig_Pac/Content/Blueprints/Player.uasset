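; Player character for a pellet-collecting pig game, with constant forward movement, score, lives and respawning.
; WASD sets an absolute heading and matching mesh yaw, and Tick feeds that heading into movement input unless the pig is dead.
; Tick also zero-pads the score string and polls pellet count and lives to open the win or game-over level.
; BeginPlay creates the HUD and caches the spawn transform that Reset restores while lives remain.
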(event `Move Pig`
  ;[0.9109 0.151 1] Move Pig per each frame ---> Infinite Movement
  (if (not (`self.Dead?`))
    (`self.AddMovementInput` (`KismetMathLibrary.Conv_RotatorToVector` (`self.Rotation`)))))

(event `Set Rotation`
  (bind _mesh (`self.Mesh`))
  ;[0.8588 0.1146 1] Initialize Rotation for Actor and Mesh
  (bind _output_get (set `self.Rotation` (`self.GetControlRotation`)))
  (set `self.Initial Rotation` _output_get)
  (`SceneComponent.K2_SetWorldRotation` _mesh (`SceneComponent.K2_GetComponentRotation` _mesh) false false))

(event `Key|W`
  (params (Key :type "Key Structure"))
  ;[1 0.1198 0.873] Turn Pig
  (:`Pressed`
    (set `self.Rotation` (struct :`Yaw` -90.0))
    (`SceneComponent.K2_SetWorldRotation` (`self.Mesh`) (struct :`Yaw` 180.0) false false)))

(event `Set UI`
  ;[0.9465 0.2031 1] Set UI
  (bind _returnvalue (`|CreateWidget` "/Game/Blueprints/Pig_UI.Pig_UI_C"))
  (`UserWidget.AddToPlayerScreen` _returnvalue 0))

(event `Key|S`
  (params (Key :type "Key Structure"))
  ;[1 0.1198 0.873] Turn Pig
  (:`Pressed`
    (set `self.Rotation` (struct :`Yaw` 90.0))
    (`SceneComponent.K2_SetWorldRotation` :`self` (`self.Mesh`))))

(event `Key|D`
  (params (Key :type "Key Structure"))
  ;[1 0.1198 0.873] Turn Pig
  (:`Pressed`
    (set `self.Rotation` (struct))
    (`SceneComponent.K2_SetWorldRotation` (`self.Mesh`) (struct :`Yaw` 270.0) false false)))

(event `self.ReceiveTick`
  (params (DeltaSeconds :type "Float (single-precision)"))
  ;[0.821 0.1198 0.9583] Ticks
  (`|ExecutionSequence`
    (:`then_0`
      (`self.Move Pig`))
    (:`then_1`
      (`self.UpdateScore`))
    (:`then_2`
      (`self.OpenCongratsScreen`))
    (:`then_3`
      (`self.OpenGameOverScreen`))))

(event `Key|A`
  (params (Key :type "Key Structure"))
  ;[1 0.1198 0.873] Turn Pig
  (:`Pressed`
    (set `self.Rotation` (struct :`Yaw` -180.0))
    (`SceneComponent.K2_SetWorldRotation` (`self.Mesh`) (struct :`Yaw` 90.0) false false)))

(event `self.ReceiveBeginPlay`
  ;[0.802 0.2015 1] Begin Play Events to Call Se Rotation, Set UI, and Calculate Level Events; and call the Initialize Player Location Function
  (`|ExecutionSequence`
    (:`then_0`
      (`self.Set Rotation`))
    (:`then_1`
      (`self.Set UI`))
    (:`then_2`
      (`self.Inialize Player Location`))))

(event `Reset`
  (bind _mesh (`self.Mesh`))
  ;[1 0.151 0.9244] Respawn Big
  (if (> (`self.Lives`) 0)
    (set `self.Dead?` false)
    (`SceneComponent.K2_SetWorldLocationAndRotation` (`self.CapsuleComponent`) (`self.Intial Location`) (`self.Initial Rotation`) false false)
    (`SceneComponent.K2_SetWorldLocationAndRotation` _mesh (`self.Intial Location`) (`SceneComponent.K2_GetComponentRotation` _mesh) false false)))

(fn `Decrement Lives`
  ;[1 1 1] Decrease Amount of Lives
  (if (> (`self.Lives`) 0)
    (`/Engine/EditorBlueprintResources/StandardMacros.DecrementInt` (`self.Lives`))))

(fn `Inialize Player Location`
  ;[1 1 1] Set The Players Initial Location to aid in Respawning
  (set `self.Intial Location` (`self.K2_GetActorLocation`)))

(fn `OpenCongratsScreen`
  ;[1 1 1] If Player Collects All Pellets
  (bind _pelletsleft (`self.PelletsLeft?`))
  (if _pelletsleft
    (`WidgetLayoutLibrary.RemoveAllWidgets`)
    (`GameplayStatics.OpenLevel` "CongratsScreen")))

(fn `OpenGameOverScreen`
  ;[1 1 1] If Player Runs Out of Lives
  (if (== (`self.Lives`) 0)
    (`WidgetLayoutLibrary.RemoveAllWidgets`)
    (`GameplayStatics.OpenLevel` "GameOver")))

(fn `PelletsLeft?`
  (returns (PelletsLeft :type Boolean))
  ;[1 1 1] Are there any Pellets Left?
  (bind _outactors (`GameplayStatics.GetAllActorsOfClass` "/Game/Blueprints/Pellet.Pellet_C"))
  (return (== (`KismetArrayLibrary.Array_Length` _outactors) 0)))

(fn `UpdateScore`
  (bind _returnvalue (`KismetStringLibrary.Len` (`self.Score_String`)))
  ;[1 1 1] Add Zeros Infront of Score
  (set `self.Score_String` (`KismetStringLibrary.Conv_IntToString` (`self.Score`)))
  (if (< _returnvalue (`self.MinDigits`))
    (for _ (range (+ (- (`self.MinDigits`) _returnvalue) 1))
      (set `self.Score_String` (`KismetStringLibrary.Concat_StrStr` "0" (`self.Score_String`))))))

(fn `UserConstructionScript`)
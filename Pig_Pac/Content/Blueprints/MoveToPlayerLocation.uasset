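; Behavior Tree task that sends the AI controller's pawn toward the first player character.
; An AI MoveTo targets the player actor, using Distance as both acceptance radius and destination offset.
; The task reports success as soon as the move is issued and again on arrival, so it does not wait for completion.
; Move failure and external aborts both call Finish Abort.
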(event `self.ReceiveExecuteAI`
  (params (OwnerController :type "AIController Object Reference") (ControlledPawn :type "Pawn Object Reference"))
  (bind _returnvalue (`GameplayStatics.GetPlayerCharacter` 0))
  (bind _distance (`self.Distance`))
  ;[1 1 1] Move To Player
  (bind _asai_controller (cast `/Game/Blueprints/AI_Controller` OwnerController))
  (`|AIMoveTo` (`Controller.K2_GetPawn` _asai_controller) (- (`Actor.K2_GetActorLocation` _returnvalue) _distance) _returnvalue (`KismetMathLibrary.Conv_IntToDouble` _distance) true
    (:`then`
      (`self.FinishExecute` true :!label _label))
    (:`OnSuccess`
      (goto _label))
    (:`OnFail`
      (`self.FinishAbort`))))

(event `self.ReceiveAbortAI`
  (params (OwnerController :type "AIController Object Reference") (ControlledPawn :type "Pawn Object Reference"))
  ;[1 1 1] Abort if False
  (`self.FinishAbort`))
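; Enemy AI controller that runs the Enemy_BT behavior tree and feeds it information about the player.
; AI perception updates set the CanSeePlayer? blackboard key from whether the stimulus was successfully sensed.
; Every tick it writes the distance from the controlled pawn to the player character into Distance, and copies the player's Dead flag into PigsDead.
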(event `self.ReceiveBeginPlay`
  ;[1 1 1] Run Behaivor Tree
  (`self.RunBehaviorTree` "/Game/Blueprints/Enemy_BT.Enemy_BT"))

(event `self.AIPerception.OnTargetPerceptionUpdated`
  (params (Actor :type "Actor Object Reference") (Stimulus :type "AIStimulus Structure"))
  ;[1 1 1] CanSeePlayer? Functionality
  (bind _output_get (set `self.CanSeePlayer?` (`.bSuccessfullySensed` (break `AIStimulus` Stimulus))))
  (`BlackboardComponent.SetValueAsBool` (`AIBlueprintHelperLibrary.GetBlackboard` null) "CanSeePlayer?" _output_get))

(event `self.ReceiveTick`
  (params (DeltaSeconds :type "Float (single-precision)"))
  (`|ExecutionSequence`
    (:`then_0`
      ;[1 1 1] Pass Distance Value from Controller to Blackboard
      (bind _distance (`self.Get Distance to Player Character`))
      (`BlackboardComponent.SetValueAsFloat` (`AIBlueprintHelperLibrary.GetBlackboard` null) "Distance" _distance))
    (:`then_1`
      ;[1 1 1] Set PigsDead
      (bind _asplayer (cast `/Game/Blueprints/Player` (`GameplayStatics.GetPlayerCharacter` 0)))
      (`BlackboardComponent.SetValueAsBool` (`AIBlueprintHelperLibrary.GetBlackboard` null) "PigsDead" (`/Game/Blueprints/Player.Dead?` _asplayer)))))

(fn `Get Distance to Player Character`
  (returns (Distance :type "Float (double-precision)"))
  ;[1 1 1] Calculate Distance between AI and Player
  (return (`self.GetDistanceTo` (`self.K2_GetPawn`) (`GameplayStatics.GetPlayerCharacter` 0))))

(fn `UserConstructionScript`)